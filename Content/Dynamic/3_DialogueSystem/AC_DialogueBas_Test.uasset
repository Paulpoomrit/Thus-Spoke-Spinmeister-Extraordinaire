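; Test dialogue component that overrides its parent's Dialogue function with a short branching placeholder conversation from a speaker named Paul.
; A YES/NO AddDialogue node branches on option index to a Happy or Sad Paul reply with a Continue option.
; Each node gates flow on its returned state, with Pass Through advancing until progress is cleared and the conversation closes.
; The first node's Updated state only prints a debug string.
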(fn `Dialogue`
  (`parent.Dialogue`)
  (bind (_state _optionindex) (`self.AddDialogue` "Paul" "Lorem ipsum odor amet, consectetuer adipiscing elit. Luctus pulvinar tristique condimentum iaculis per auctor. Eros quis ligula nostra eleifend nisl tempor; dolor malesuada. Inceptos odio penatibus auctor purus magnis eleifend eros. Cubilia facilisis ullamcorper nam potenti egestas mauris luctus. Inceptos suspendisse finibus himenaeos aliquam dignissim egestas?" (`|MakeArray` "YES" "NO" :!type "Text")))
  (switch `/Game/Dynamic/3_DialogueSystem/E_DialogueState` _state
    (:`NewEnumerator0`
      (switch `int` _optionindex
        (:`0`
          (bind _state_2 (`self.AddDialogue` "Happy Paul" "nceptos odio penatibus auctor purus magnis eleifend eros. Cubilia facilisis ullamcorper nam potenti egestas mauris luctus. Inceptos suspendisse finibus himenaeos aliquam dignissim egestas?" (`|MakeArray` "Continue" :!type "Text")))
          (switch `/Game/Dynamic/3_DialogueSystem/E_DialogueState` _state_2
            (:`NewEnumerator0`
              (`self.ClearDialogueProgress`)
              (`self.CloseConversation`))))
        (:`1`
          (bind _state_3 (`self.AddDialogue` "Sad Paul" "Inceptos suspendisse finibus himenaeos aliquam dignissim egestas?" (`|MakeArray` "Continue" :!type "Text")))
          (switch `/Game/Dynamic/3_DialogueSystem/E_DialogueState` _state_3
            (:`NewEnumerator0`
              (`self.ClearDialogueProgress`)
              (`self.CloseConversation`))))))
    (:`NewEnumerator1`
      (`KismetSystemLibrary.PrintString` "FUCK"))))