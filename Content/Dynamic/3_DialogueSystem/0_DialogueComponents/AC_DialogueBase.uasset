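; Base dialogue component that runs branching conversations through a WBP_Dialogue widget and notifies its owner when they close.
; Child classes script conversations by overriding the empty Dialogue function with AddDialogue calls.
; Each selection is saved by step index and Dialogue reruns from the start, with answered steps returning stored options and unanswered ones updating the widget.
; Helpers clear or rewind progress, switch dialogue trees, and trigger the player character's spin.
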(fn `AddDialogue`
  (params (Speaker :type Text) (Dialogue :type Text) (OptionText :type "Array of Text"))
  (returns (State :type "/Game/Dynamic/3_DialogueSystem/E_DialogueState Enum") (OptionIndex :type Integer))
  (bind _dialogueindex (`self.DialogueIndex`))
  (bind (_value _returnvalue) (`BlueprintMapLibrary.Map_Find` (`self.DialogueProgress`) _dialogueindex))
  (`/Engine/EditorBlueprintResources/StandardMacros.IncrementInt` _dialogueindex
    (:`  `
      (if _returnvalue
        (return "NewEnumerator0" _value)
        (else
          (`/Game/Dynamic/3_DialogueSystem/WBP_Dialogue.UpdateDialogueText` (`self.DialogueWidget`) (`self.DialogueIndex`) (`local.Speaker`) (`local.Dialogue`) (`local.OptionText`))
          (return "NewEnumerator1" 0))))))

(fn `ClearDialogueProgress`
  (`BlueprintMapLibrary.Map_Clear` (`self.DialogueProgress`)))

(fn `CloseConversation`
  (bind _returnvalue (`GameplayStatics.GetPlayerController` 0))
  (`Widget.RemoveFromParent` (`self.DialogueWidget`))
  (`WidgetBlueprintLibrary.SetInputMode_GameOnly` _returnvalue)
  (set `PlayerController.bShowMouseCursor` false _returnvalue)
  (message `/Game/Dynamic/3_DialogueSystem/BPI_Interactable.ConversationClosed` (`self.GetOwner`)))

(fn `Dialogue`)

(fn `OpenConversation`
  (bind _returnvalue (`|CreateWidget` "/Game/Dynamic/3_DialogueSystem/WBP_Dialogue.WBP_Dialogue_C" (`GameplayStatics.GetPlayerController` 0) self))
  (bind _output_get (set `self.DialogueWidget` _returnvalue))
  (`UserWidget.AddToViewport` _output_get 0)
  (`self.ProgressDialogue`))

(fn `ProgressDialogue`
  (set `self.DialogueIndex` -1)
  (`self.Dialogue`))

(fn `RemoveDialogueProgress`
  (params (ProgressSteps :type Integer))
  (for _index (range (+ ProgressSteps 1))
    (`BlueprintMapLibrary.Map_Remove` (`self.DialogueProgress`) (- (`self.DialogueIndex`) _index))))

(fn `SetDialogueTreeIndex`
  (params (DialogueTreeIndex :type Integer))
  (set `self.DialogueTreeIndex` DialogueTreeIndex)
  (`self.ClearDialogueProgress`))

(fn `StartSpinningComp`
  (bind _asbp_paper_char_base (cast `/Game/Dynamic/1_Blueprints/1_PaperCharBase/BP_PaperCharBase` (`GameplayStatics.GetPlayerCharacter` 0)))
  (`/Game/Dynamic/1_Blueprints/1_PaperCharBase/BP_PaperCharBase.EventStartSpinning` _asbp_paper_char_base))

(fn `UpdateSelected`
  (params (ProgressIndex :type "Integer (by ref)") (OptionIndex :type "Integer (by ref)"))
  (`BlueprintMapLibrary.Map_Add` (`self.DialogueProgress`) ProgressIndex OptionIndex)
  (`self.ProgressDialogue`))