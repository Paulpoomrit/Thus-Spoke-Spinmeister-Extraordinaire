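; Dialogue component for a satirical press exchange in which a news reporter challenges the Spinmeister over an ally's war in the Middle East.
; The Dialogue function hardcodes the conversation as nested AddDialogue calls, branching on returned state and option index.
; After linear opening lines, the player picks one of three deflections, each playing its own reply before calling StartSpinningComp.
; AddDialogue and CloseConversation overrides only forward to the parent.
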(fn `AddDialogue`
  (params (Speaker :type Text) (Dialogue :type Text) (OptionText :type "Array of Text (by ref)"))
  (returns (State :type "/Game/Dynamic/3_DialogueSystem/E_DialogueState Enum") (OptionIndex :type Integer))
  (bind (_state _optionindex) (`parent.AddDialogue` Speaker Dialogue OptionText))
  (return _state _optionindex))

(fn `CloseConversation`
  (`parent.CloseConversation`))

(fn `Dialogue`
  (bind (_state _optionindex) (`self.AddDialogue` "News Reporter 2" "Sir, people are saying that “our ally in the Middle East”’s scale and cruelty of retaliation is now tantamount to genocide." (`|MakeArray` "CONTINUE" :!type "Text")))
  (switch `/Game/Dynamic/3_DialogueSystem/E_DialogueState` _state
    (:`NewEnumerator0`
      (switch `int` _optionindex
        (:`0`
          (bind (_state_2 _optionindex_2) (`self.AddDialogue` "News Reporter 2" "And what Amerika is doing is enabling and condoning them to continue the apartheid that has been going on for over a century!" (`|MakeArray` "CONTINUE" :!type "Text")))
          (switch `/Game/Dynamic/3_DialogueSystem/E_DialogueState` _state_2
            (:`NewEnumerator0`
              (switch `int` _optionindex_2
                (:`0`
                  (bind (_state_3 _optionindex_3) (`self.AddDialogue` "Spinmeister" "Well, using the words “apartheid” or “genocide” might not be factually correct here." (`|MakeArray` "CONTINUE" :!type "Text")))
                  (switch `/Game/Dynamic/3_DialogueSystem/E_DialogueState` _state_3
                    (:`NewEnumerator0`
                      (switch `int` _optionindex_3
                        (:`0`
                          (bind (_state_4 _optionindex_4) (`self.AddDialogue` "Spinmeister" "Also, I have to remind you that this is a particularly very complex topic to touch on historically, and…" (`|MakeArray` "Don’t be woke!" "They deserve it." "Don’t be antisemitic." :!type "Text")))
                          (switch `/Game/Dynamic/3_DialogueSystem/E_DialogueState` _state_4
                            (:`NewEnumerator0`
                              (switch `int` _optionindex_4
                                (:`0`
                                  (bind (_state_5 _optionindex_5) (`self.AddDialogue` "Spinmeister" "Saying “colonialism bad” and just trying to be woke don’t really convey such complexity at all. And…" (`|MakeArray` "CONTINUE" :!type "Text")))
                                  (switch `/Game/Dynamic/3_DialogueSystem/E_DialogueState` _state_5
                                    (:`NewEnumerator0`
                                      (switch `int` _optionindex_5
                                        (:`0`
                                          (`self.StartSpinningComp`))))))
                                (:`1`
                                  (bind (_state_6 _optionindex_6) (`self.AddDialogue` "Spinmeister" "They bring this upon themselves after the attack of October 7th. And…" (`|MakeArray` "CONTINUE" :!type "Text")))
                                  (switch `/Game/Dynamic/3_DialogueSystem/E_DialogueState` _state_6
                                    (:`NewEnumerator0`
                                      (switch `int` _optionindex_6
                                        (:`0`
                                          (`self.StartSpinningComp`))))))
                                (:`2`
                                  (bind (_state_7 _optionindex_7) (`self.AddDialogue` "Spinmeister" "Zionism is Judaism! Don’t be antisemitic, you woke moralists. And…" (`|MakeArray` "CONTINUE" :!type "Text")))
                                  (switch `/Game/Dynamic/3_DialogueSystem/E_DialogueState` _state_7
                                    (:`NewEnumerator0`
                                      (switch `int` _optionindex_7
                                        (:`0`
                                          (`self.StartSpinningComp`))))))))))))))))))))))