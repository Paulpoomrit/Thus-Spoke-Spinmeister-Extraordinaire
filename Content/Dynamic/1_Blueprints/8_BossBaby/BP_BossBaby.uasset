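; BP_BossBaby is a boss Blueprint that shows its own on-screen health bar and can turn to face the player.
; On BeginPlay it creates a WBP_BossBar widget, then every Tick sets that bar from its health percentage, alongside the parent class logic.
; RotateTowardsPlayer smoothly interpolates yaw toward the first player character with RInterpTo; nothing in this file calls it.
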(event `self.ReceiveBeginPlay`
  (`parent.ReceiveBeginPlay`)
  (bind _returnvalue (`|CreateWidget` "/Game/Dynamic/1_Blueprints/8_BossBaby/WBP_BossBar.WBP_BossBar_C"))
  (`UserWidget.AddToViewport` _returnvalue 0)
  (set `self.HealthBarWidget` _returnvalue))

(event `self.ReceiveTick`
  (params (DeltaSeconds :type "Float (single-precision)"))
  (`parent.ReceiveTick` DeltaSeconds)
  (`/Game/Dynamic/1_Blueprints/8_BossBaby/TPWBP_StatusBar.SetStatusBarPercent` (`/Game/Dynamic/1_Blueprints/8_BossBaby/WBP_BossBar.TPWBP_StatusBar` (`self.HealthBarWidget`)) (`self.GetHealthPercentage`)))

(fn `RotateTowardsPlayer`
  (bind (_returnvalue_roll _returnvalue_pitch _returnvalue_yaw) (`KismetMathLibrary.BreakRotator` (`KismetMathLibrary.RInterpTo` (`self.K2_GetActorRotation`) (`KismetMathLibrary.FindLookAtRotation` (`self.K2_GetActorLocation`) (`self.K2_GetActorLocation` (`GameplayStatics.GetPlayerCharacter` 0))) (`GameplayStatics.GetWorldDeltaSeconds`) (`self.Interp Speed`))))
  (`self.K2_SetActorRotation` (`KismetMathLibrary.MakeRotator` 0.0 0.0 _returnvalue_yaw))
  (return))

(fn `UserConstructionScript`
  (`parent.UserConstructionScript`))