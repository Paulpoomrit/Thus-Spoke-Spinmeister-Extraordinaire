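; BP_Baby is an enemy with a Paper2D flipbook that smoothly turns to face player 0 every Tick via RInterpTo.
; UpdateFBAccordingToPlayer uses forward and right dot products to bucket the player's relative angle by side and 45-degree steps.
; Each bucket sets the sprite's relative rotation and a directional walk flipbook from FBWalkArray.
; Nothing in this graph calls that selection, and the attack/walk flipbook nodes in EventGraph are unconnected.
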(event `self.ReceiveTick`
  (params (DeltaSeconds :type "Float (single-precision)"))
  (`self.RotateTowardsPlayer`))

(event `self.ReceiveAnyDamage`
  (params (Damage :type "Float (single-precision)") (DamageType :type "DamageType Object Reference") (InstigatedBy :type "Controller Object Reference") (DamageCauser :type "Actor Object Reference")))

(fn `RotateTowardsPlayer`
  (`self.K2_SetActorRotation` (`KismetMathLibrary.RInterpTo` (`self.K2_GetActorRotation`) (`KismetMathLibrary.FindLookAtRotation` (`self.K2_GetActorLocation`) (`self.K2_GetActorLocation` (`GameplayStatics.GetPlayerCharacter` 0))) (`GameplayStatics.GetWorldDeltaSeconds`) (`self.Interp Speed`)))
  (return))

(fn `UpdateFBAccordingToPlayer`
  (locals (condition :type Boolean))
  (bind _returnvalue (`KismetMathLibrary.Normal` (- (`self.K2_GetActorLocation` (`GameplayStatics.GetPlayerCharacter` 0)) (`self.K2_GetActorLocation`))))
  ;[1 1 1] Find dot product to determine the angle (i.e., how much does the Baby and the player facing the same way?)
  (set `self.Degree` (`KismetMathLibrary.DegAcos` (`KismetMathLibrary.Dot_VectorVector` (`self.GetActorForwardVector`) _returnvalue)))
  ;[1 1 1] True if on the left side of the enemy./ false otherwise
  (if (< (`KismetMathLibrary.Dot_VectorVector` (`self.GetActorRightVector`) _returnvalue) 0.0)
    (`/Engine/EditorBlueprintResources/StandardMacros.CompareFloat` (`self.Degree`) 180.0
      (:`>`
        (`self.SetFlipbookWithNewRotatorAndFBIndex` (struct :`Yaw` -90.0) :!label _label))
      (:`==`
        (goto _label))
      (:`<`
        (`/Engine/EditorBlueprintResources/StandardMacros.CompareFloat` (`self.Degree`) 135.0
          (:`>`
            (`self.SetFlipbookWithNewRotatorAndFBIndex` (struct :`Yaw` 135.0) 3 :!label _label_2))
          (:`==`
            (goto _label_2))
          (:`<`
            (`/Engine/EditorBlueprintResources/StandardMacros.CompareFloat` (`self.Degree`) 90.0
              (:`>`
                (`self.SetFlipbookWithNewRotatorAndFBIndex` (struct :`Yaw` 180.0) 2 :!label _label_3))
              (:`==`
                (goto _label_3))
              (:`<`
                (`/Engine/EditorBlueprintResources/StandardMacros.CompareFloat` (`self.Degree`) 45.0
                  (:`>`
                    _)
                  (:`==`
                    _)
                  (:`<`
                    (goto _label)))
                (`self.SetFlipbookWithNewRotatorAndFBIndex` (struct :`Yaw` 45.0) 1)))))))
    (else
      (`/Engine/EditorBlueprintResources/StandardMacros.CompareFloat` (`self.Degree`) 180.0
        (:`>`
          (`self.SetFlipbookWithNewRotatorAndFBIndex` (struct :`Yaw` -45.0) 7 :!label _label_4))
        (:`==`
          (goto _label_4))
        (:`<`
          (`/Engine/EditorBlueprintResources/StandardMacros.CompareFloat` (`self.Degree`) 135.0
            (:`>`
              (`self.SetFlipbookWithNewRotatorAndFBIndex` (struct :`Yaw` 90.0) 4 :!label _label_5))
            (:`==`
              (goto _label_5))
            (:`<`
              (`/Engine/EditorBlueprintResources/StandardMacros.CompareFloat` (`self.Degree`) 90.0
                (:`>`
                  (`self.SetFlipbookWithNewRotatorAndFBIndex` (struct :`Yaw` 45.0) 5 :!label _label_6))
                (:`==`
                  (goto _label_6))
                (:`<`
                  (`/Engine/EditorBlueprintResources/StandardMacros.CompareFloat` (`self.Degree`) 45.0
                    (:`>`
                      _)
                    (:`==`
                      _)
                    (:`<`
                      (goto _label_4)))
                  (`self.SetFlipbookWithNewRotatorAndFBIndex` (struct) 6))))))))))

(fn `UserConstructionScript`)