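; BP_DerivedBabyBoss is a derived Blueprint for a baby boss enemy that adds logic to face the player.
; RotateTowardsPlayer uses RInterpTo at InterpSpeed to ease toward the look-at rotation to player 0's character, applying only yaw.
; The event graph holds only disabled stubs and the construction script just calls the parent, so nothing in this file calls the rotation function.
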(fn `RotateTowardsPlayer`
  (bind (_returnvalue_roll _returnvalue_pitch _returnvalue_yaw) (`KismetMathLibrary.BreakRotator` (`KismetMathLibrary.RInterpTo` (`self.K2_GetActorRotation`) (`KismetMathLibrary.FindLookAtRotation` (`self.K2_GetActorLocation`) (`self.K2_GetActorLocation` (`GameplayStatics.GetPlayerCharacter` 0))) (`GameplayStatics.GetWorldDeltaSeconds`) (`self.Interp Speed`))))
  (`self.K2_SetActorRotation` (`KismetMathLibrary.MakeRotator` 0.0 0.0 _returnvalue_yaw))
  (return))

(fn `UserConstructionScript`
  (`parent.UserConstructionScript`))