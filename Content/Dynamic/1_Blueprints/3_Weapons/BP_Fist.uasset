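; BP_Fist is a fist weapon Blueprint that performs an animated punch as its attack.
; StartShooting passes through a DoOnce gate, calls FireWeapon and switches the weapon's Paper2D flipbook to the punch animation.
; After a delay equal to the flipbook's length, it restores the idle flipbook and calls ResetPunch to reopen the gate, so punches cannot overlap.
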(event `self.StartShooting`
  (bind _weaponflipbook (`self.WeaponFlipbook`))
  (`/Engine/EditorBlueprintResources/StandardMacros.DoOnce` false :!label _label
    (:`Completed`
      (`self.FireWeapon` 0)
      (`PaperFlipbookComponent.SetFlipbook` _weaponflipbook "/Game/Static/RetroFPSAssets/Weapons/Punch/FB_PunchAttack.FB_PunchAttack")
      (`KismetSystemLibrary.Delay` (`PaperFlipbookComponent.GetFlipbookLength` _weaponflipbook))
      (`PaperFlipbookComponent.SetFlipbook` _weaponflipbook "/Game/Static/RetroFPSAssets/Weapons/Punch/FB_PunchIdle.FB_PunchIdle")
      (`self.ResetPunch`))))

(event `ResetPunch`
  (goto _label :!via `Reset`))

(fn `UserConstructionScript`
  (`parent.UserConstructionScript`))