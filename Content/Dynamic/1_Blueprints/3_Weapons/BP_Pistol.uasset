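; BP_Pistol is a pistol weapon that animates with Paper2D flipbooks and reports ammo to the player's HUD.
; StartShooting checks ammo, then calls FireWeapon, plays the shoot flipbook and refreshes the bullet count on the first-person character's HUD, or prints an out-of-ammo message.
; A DoOnce gate blocks refiring until the flipbook's length has elapsed, when ResetWeapon reopens it and the idle flipbook returns.
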(event `self.StartShooting`
  (bind _weaponflipbook (`self.WeaponFlipbook`))
  (bind _returnvalue (`self.HasEnoughAmmo`))
  (if _returnvalue
    (`/Engine/EditorBlueprintResources/StandardMacros.DoOnce` false :!label _label
      (:`Completed`
        (`self.FireWeapon` 1)
        (`PaperFlipbookComponent.SetFlipbook` _weaponflipbook "/Game/Static/RetroFPSAssets/Weapons/Pistol/FB_PistolShoot.FB_PistolShoot")
        (`self.UpdateUI`)
        (`KismetSystemLibrary.Delay` (`PaperFlipbookComponent.GetFlipbookLength` _weaponflipbook))
        (`PaperFlipbookComponent.SetFlipbook` (`self.WeaponFlipbook`) "/Game/Static/RetroFPSAssets/Weapons/Pistol/FB_PistolIdle.FB_PistolIdle")
        (`self.ResetWeapon`)))
    (else
      (`KismetSystemLibrary.PrintString` "Out of Ammo!"))))

(event `ResetWeapon`
  (goto _label :!via `Reset`))

(event `self.UpdateUI`
  (bind _asbp_first_person_character (cast `/Game/Dynamic/FirstPerson/Blueprints/BP_FirstPersonCharacter` (`GameplayStatics.GetPlayerCharacter` 0)))
  (`/Game/Dynamic/1_Blueprints/4_UI/W_PlayerHUD.UpdateBulletAmmo` (`/Game/Dynamic/FirstPerson/Blueprints/BP_FirstPersonCharacter.PlayerHUD` _asbp_first_person_character)))

(fn `UserConstructionScript`
  (`parent.UserConstructionScript`))