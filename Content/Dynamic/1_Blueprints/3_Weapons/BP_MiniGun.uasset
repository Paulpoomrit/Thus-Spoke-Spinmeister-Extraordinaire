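; BP_MiniGun is an automatic minigun weapon that fires repeatedly while shooting is active.
; StartShooting passes a DoOnce gate to start a looping timer, which checks ammo, fires, switches the sprite flipbook to firing and refreshes the player HUD's ammo display.
; StopShooting or running out of ammo clears the timer, restores the idle flipbook and resets the gate.
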(event `self.StartShooting`
  (`/Engine/EditorBlueprintResources/StandardMacros.DoOnce` false :!label _label
    (:`Completed`
      (bind _returnvalue (`KismetSystemLibrary.K2_SetTimerDelegate` (delegate `FireMiniGun`) 0.15 true))
      (set `self.MiniGunEvent` _returnvalue))))

(event `ResetMiniGun`
  (goto _label :!via `Reset`))

(event `FireMiniGun`
  (bind _returnvalue (`self.HasEnoughAmmo`))
  (if _returnvalue
    (`self.FireWeapon` 1)
    (`PaperFlipbookComponent.SetFlipbook` (`self.WeaponFlipbook`) "/Game/Static/RetroFPSAssets/Weapons/MiniGun/FB_SubmachinegunFire.FB_SubmachinegunFire")
    (`self.UpdateUI`)
    (else
      (`KismetSystemLibrary.PrintString` "Out of Ammo!")
      (`KismetSystemLibrary.K2_ClearAndInvalidateTimerHandle` (`self.MiniGunEvent`) :!label _label_2)
      (`PaperFlipbookComponent.SetFlipbook` (`self.WeaponFlipbook`) "/Game/Static/RetroFPSAssets/Weapons/MiniGun/FB_SubmachinegunIdle.FB_SubmachinegunIdle")
      (`self.ResetMiniGun`))))

(event `self.StopShooting`
  (goto _label_2))

(event `self.UpdateUI`
  (bind _asbp_first_person_character (cast `/Game/Dynamic/FirstPerson/Blueprints/BP_FirstPersonCharacter` (`GameplayStatics.GetPlayerCharacter` 0)))
  (`/Game/Dynamic/1_Blueprints/4_UI/W_PlayerHUD.UpdateBulletAmmo` (`/Game/Dynamic/FirstPerson/Blueprints/BP_FirstPersonCharacter.PlayerHUD` _asbp_first_person_character)))

(fn `UserConstructionScript`
  (`parent.UserConstructionScript`))