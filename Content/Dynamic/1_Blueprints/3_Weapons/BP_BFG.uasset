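; BP_BFG is the BFG weapon Blueprint, firing a projectile when the player character has at least 30 cells.
; StartShooting passes a DoOnce gate, plays the fire flipbook and waits for its length before calling FireWeapon with 30 and FireProjectile.
; It then restores the idle flipbook, refreshes the HUD cell ammo and resets the gate, blocking overlapping shots during the animation.
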(event `self.StartShooting`
  (bind _weaponflipbook (`self.WeaponFlipbook`))
  (if (>= (`FirstPersonCharacter.CurrentCell` (`self.FirstPersonCharacterRef`)) 30)
    (`/Engine/EditorBlueprintResources/StandardMacros.DoOnce` false :!label _label
      (:`Completed`
        (`PaperFlipbookComponent.SetFlipbook` _weaponflipbook "/Game/Static/RetroFPSAssets/Weapons/BFG/BP_BFGFire.BP_BFGFire")
        (`KismetSystemLibrary.Delay` (`PaperFlipbookComponent.GetFlipbookLength` _weaponflipbook))
        (`self.FireWeapon` 30)
        (`self.FireProjectile`)
        (`PaperFlipbookComponent.SetFlipbook` _weaponflipbook "/Game/Static/RetroFPSAssets/Weapons/BFG/BP_BFGIdle.BP_BFGIdle")
        (`self.UpdateUI`)
        (`self.ResetBFG`)))))

(event `ResetBFG`
  (goto _label :!via `Reset`))

(event `self.UpdateUI`
  (bind _asbp_first_person_character (cast `/Game/Dynamic/FirstPerson/Blueprints/BP_FirstPersonCharacter` (`GameplayStatics.GetPlayerCharacter` 0)))
  (`/Game/Dynamic/1_Blueprints/4_UI/W_PlayerHUD.UpdateCellAmmo` (`/Game/Dynamic/FirstPerson/Blueprints/BP_FirstPersonCharacter.PlayerHUD` _asbp_first_person_character)))

(fn `UserConstructionScript`
  (`parent.UserConstructionScript`))