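; Weapon pickup that shows a 2D sprite and hands its weapon to the first-person player character on contact.
; The construction script maps the Weapon selection to a Paper sprite and a matching weapon class.
; Each tick it yaws toward the player, billboard-style.
; When BP_FirstPersonCharacter overlaps its sphere, it passes the class to PickUpWeapon and destroys itself.
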(event `self.ReceiveTick`
  (params (DeltaSeconds :type "Float (single-precision)"))
  (bind (_returnvalue_roll _returnvalue_pitch _returnvalue_yaw) (`KismetMathLibrary.BreakRotator` (`KismetMathLibrary.FindLookAtRotation` (`self.K2_GetActorLocation`) (`self.K2_GetActorLocation` (`GameplayStatics.GetPlayerCharacter` 0)))))
  ;[1 1 1] Make The Pickable Weapon Yaw Follows the Player
  (`self.K2_SetActorRotation` (`KismetMathLibrary.MakeRotator` 0.0 0.0 _returnvalue_yaw)))

(event `self.Sphere.OnComponentBeginOverlap`
  (params (OverlappedComponent :type "PrimitiveComponent Object Reference") (OtherActor :type "Actor Object Reference") (OtherComp :type "PrimitiveComponent Object Reference") (OtherBodyIndex :type Integer) (bFromSweep :type Boolean) (SweepResult :type "HitResult Structure (by ref)"))
  ;[1 1 1] Pick Up the Weapon
  (bind _asbp_first_person_character (cast `/Game/Dynamic/FirstPerson/Blueprints/BP_FirstPersonCharacter` OtherActor))
  (`/Game/Dynamic/FirstPerson/Blueprints/BP_FirstPersonCharacter.PickUpWeapon` _asbp_first_person_character (`self.WeaponClass`))
  (`self.K2_DestroyActor`))

(fn `UserConstructionScript`
  (switch `/Game/Dynamic/1_Blueprints/3_Weapons/E_PickableWeapon` (`self.Weapon`)
    (:`NewEnumerator0`
      (`PaperSpriteComponent.SetSprite` (`self.PaperSprite`) "/Game/Static/RetroFPSAssets/Weapons/Shotgun/S_Shotgun.S_Shotgun")
      (set `self.WeaponClass` "/Game/Dynamic/1_Blueprints/3_Weapons/BP_Shotgun.BP_Shotgun_C"))
    (:`NewEnumerator1`
      (`PaperSpriteComponent.SetSprite` (`self.PaperSprite`) "/Game/Static/RetroFPSAssets/Weapons/MiniGun/S_MiniGun.S_MiniGun")
      (set `self.WeaponClass` "/Game/Dynamic/1_Blueprints/3_Weapons/BP_MiniGun.BP_MiniGun_C"))
    (:`NewEnumerator2`
      (`PaperSpriteComponent.SetSprite` (`self.PaperSprite`) "/Game/Static/RetroFPSAssets/Weapons/PlasmaGun/S_PlasmaGun.S_PlasmaGun")
      (set `self.WeaponClass` "/Game/Dynamic/1_Blueprints/3_Weapons/BP_PlasmaGun.BP_PlasmaGun_C"))
    (:`NewEnumerator3`
      (`PaperSpriteComponent.SetSprite` (`self.PaperSprite`) "/Game/Static/RetroFPSAssets/Weapons/RPG/S_RPG.S_RPG")
      (set `self.WeaponClass` "/Game/Dynamic/1_Blueprints/3_Weapons/BP_RPG.BP_RPG_C"))
    (:`NewEnumerator4`
      (`PaperSpriteComponent.SetSprite` (`self.PaperSprite`) "/Game/Static/RetroFPSAssets/Weapons/BFG/S_BFG.S_BFG")
      (set `self.WeaponClass` "/Game/Dynamic/1_Blueprints/3_Weapons/BP_BFG.BP_BFG_C"))
    (:`NewEnumerator5`
      (`PaperSpriteComponent.SetSprite` (`self.PaperSprite`) "/Game/Static/RetroFPSAssets/Weapons/Chainsaw/S_Chainsaw.S_Chainsaw")
      (set `self.WeaponClass` "/Game/Dynamic/1_Blueprints/3_Weapons/BP_Chainsaw.BP_Chainsaw_C"))))