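; Chainsaw weapon Blueprint that attacks repeatedly while shooting is active, using flipbook sprites for its attack and idle looks.
; StartShooting passes a DoOnce gate to start a looping timer, whose ticks call FireWeapon, show the attack flipbook and refresh the player HUD's bullet ammo.
; StopShooting clears the timer, restores the idle flipbook and resets the gate for the next press.
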(event `self.StartShooting`
  (`/Engine/EditorBlueprintResources/StandardMacros.DoOnce` false :!label _label
    (:`Completed`
      (bind _returnvalue (`KismetSystemLibrary.K2_SetTimerDelegate` (delegate `ChainsawAttack`) 0.15 true))
      (set `self.ChainsawEvent` _returnvalue))))

(event `ResetChainsaw`
  (goto _label :!via `Reset`))

(event `ChainsawAttack`
  (`self.FireWeapon` 0)
  (`PaperFlipbookComponent.SetFlipbook` (`self.WeaponFlipbook`) "/Game/Static/RetroFPSAssets/Weapons/Chainsaw/FB_ChainsawAttack.FB_ChainsawAttack")
  (`self.UpdateUI`))

(event `self.StopShooting`
  (`KismetSystemLibrary.K2_ClearAndInvalidateTimerHandle` (`self.ChainsawEvent`))
  (`PaperFlipbookComponent.SetFlipbook` (`self.WeaponFlipbook`) "/Game/Static/RetroFPSAssets/Weapons/Chainsaw/FB_ChainsawIdle.FB_ChainsawIdle")
  (`self.ResetChainsaw`))

(event `self.UpdateUI`
  (bind _asbp_first_person_character (cast `/Game/Dynamic/FirstPerson/Blueprints/BP_FirstPersonCharacter` (`GameplayStatics.GetPlayerCharacter` 0)))
  (`/Game/Dynamic/1_Blueprints/4_UI/W_PlayerHUD.UpdateBulletAmmo` (`/Game/Dynamic/FirstPerson/Blueprints/BP_FirstPersonCharacter.PlayerHUD` _asbp_first_person_character)))

(fn `UserConstructionScript`
  (`parent.UserConstructionScript`))