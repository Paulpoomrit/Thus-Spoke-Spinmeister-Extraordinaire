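; Base 2D paper character that drives jump and landing animation and starts interactions with dialogue and spin spaces.
; Jump and land events jump nodes in the Movement animation state machine, and BeginPlay adds a spinning overlay widget to the viewport.
; Overlapping a BP_DialogueSpace or BP_SpinSpace calls its Interact, then switches to UI-only input with a visible cursor.
; ConversationClosed restores game-only input and hides the cursor.
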(event `self.ReceiveBeginPlay`
  (bind _returnvalue (`|CreateWidget` "/Game/Dynamic/3_DialogueSystem/WBP_SpinningOverlay.WBP_SpinningOverlay_C"))
  (`UserWidget.AddToViewport` _returnvalue 0))

(event `self.OnJumped`
  (`PaperZDAnimInstance.JumpToNode` (`PaperZDAnimationComponent.AnimInstance` (`self.AnimationComponent`)) "Airborne" "Movement"))

(event `self.OnLanded`
  (params (Hit :type "HitResult Structure (by ref)"))
  (`PaperZDAnimInstance.JumpToNode` (`PaperZDAnimationComponent.AnimInstance` (`self.AnimationComponent`)) "Land" "Movement"))

(event `self.ReceiveActorBeginOverlap`
  (params (OtherActor :type "Actor Object Reference"))
  (bind _returnvalue (`GameplayStatics.GetPlayerController` 0))
  (bind _returnvalue_2 (`GameplayStatics.GetPlayerController` 0))
  (`KismetSystemLibrary.PrintString` "Overlap")
  (bind _asbp_dialogue_space (cast `/Game/Dynamic/3_DialogueSystem/BP_DialogueSpace` OtherActor)
    (:`then`
      (`KismetSystemLibrary.PrintString` "cast sucess")
      (`/Game/Dynamic/3_DialogueSystem/BPI_Interactable.Interact` _asbp_dialogue_space self)
      (`WidgetBlueprintLibrary.SetInputMode_UIOnlyEx` _returnvalue_2 null "DoNotLock" true)
      (set `PlayerController.bShowMouseCursor` true _returnvalue_2))
    (:`CastFailed`
      (bind _asbp_spin_space (cast `/Game/Dynamic/3_DialogueSystem/SpinningMechanics/BP_SpinSpace` OtherActor))
      (`/Game/Dynamic/3_DialogueSystem/BPI_Interactable.Interact` _asbp_spin_space self)
      (`WidgetBlueprintLibrary.SetInputMode_UIOnlyEx` _returnvalue null "DoNotLock" true)
      (set `PlayerController.bShowMouseCursor` true _returnvalue))))

(event `/Game/Dynamic/3_DialogueSystem/BPI_Interactable.ConversationClosed`
  (bind _returnvalue (`GameplayStatics.GetPlayerController` 0))
  (set `PlayerController.bShowMouseCursor` false _returnvalue)
  (`WidgetBlueprintLibrary.SetInputMode_GameOnly` _returnvalue true))

(fn `UserConstructionScript`)